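; Thrown grenade projectile that detonates after a fuse timer, or on hitting listed actor classes when impact explosion is enabled.
; Bounces play surface-specific sounds.
; Boom plays sound and FX, then a timeline grows the blast sphere before destroying the actor.
; Overlaps send explosion messages to filtered actors, damaging the owning player only with friendly fire, and a radial impulse targets destructibles.
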(event OnComponentBeginOverlap(ExplosionSphere)
  (params (OverlappedComponent :type Primitive%20Component%20Object%20Reference) (OtherActor :type Actor%20Object%20Reference) (OtherComp :type Primitive%20Component%20Object%20Reference) (OtherBodyIndex :type Integer) (bFromSweep :type Boolean) (SweepResult :type Hit%20Result%20Structure%20%28by%20ref%29))
  ;[1 0 0] Explosion Radius Overlap
  (if (Variables|Boolean|GetHasDetonate)
    (CallFunction|ExplosionRadiusOverlap OtherActor (Variables|Grenade|GetGrenadeLocation))))

(event OnComponentHit(GrenadeMesh)
  (params (HitComponent :type Primitive%20Component%20Object%20Reference) (OtherActor :type Actor%20Object%20Reference) (OtherComp :type Primitive%20Component%20Object%20Reference) (NormalImpulse :type Vector :default "0, 0, 0") (Hit :type Hit%20Result%20Structure%20%28by%20ref%29))
  (bind _returnvalue (Transformation|GetActorLocation))
  ;[1 0 1] Event Hit
  ;[0.1053 1 0] Play Rebound Sound
  (switch Utilities|FlowControl|Switch|SwitchonEPhysicalSurface (Variables|/Script/PhysicsCore.PhysicalMaterial|GetSurfaceType (.PhysMat (Collision|BreakHitResult Hit)))
    (:SurfaceType_Default
      (Audio|PlaySoundatLocation "/Game/SFX/MC/WEAPON/ATTACK/GRENADE/SFX_MC_WEA_ATK_Grenade_ReboundDirt/SFX_MC_WEA_GrenadeReboundDirt_V01.SFX_MC_WEA_GrenadeReboundDirt_V01" _returnvalue "0, 0, 0" 1.0 1.0 0.0 0 0 0))
    (:SurfaceType1
      (Audio|PlaySoundatLocation "/Game/SFX/MC/WEAPON/ATTACK/GRENADE/SFX_MC_WEA_ATK_Grenade_ReboundRock/SFX_MC_WEA_GrenadeREboundRock_V01.SFX_MC_WEA_GrenadeReboundRock_V01" _returnvalue "0, 0, 0" 1.0 1.0 0.0 0 0 0))
    (:SurfaceType2
      (Audio|PlaySoundatLocation "/Game/SFX/MC/WEAPON/ATTACK/GRENADE/SFX_MC_WEA_ATK_Grenade_ReboundWood/SFX_MX_WEA_GrenadeReboundWood_V01.SFX_MX_WEA_GrenadeReboundWood_V01" _returnvalue "0, 0, 0" 1.0 1.0 0.0 0 0 0))
    (:SurfaceType5
      (Audio|PlaySoundatLocation "/Game/SFX/MC/WEAPON/ATTACK/GRENADE/SFX_MC_WEA_ATK_Grenade_ReboundMetal/SFX_MC_WEA_GrenadeReboundMetal_V01.SFX_MC_WEA_GrenadeReboundMetal_V01" _returnvalue "0, 0, 0" 1.0 1.0 0.0 0 0 0)))
  ;[1 0 0] Check actor is overlap
  (if (Variables|Boolean|GetExplosionOnImpact)
    (if (Utilities|Array|ContainsItem (Variables|Grenade|GetActorsExploseOnImpact) (Utilities|GetClass OtherActor))
      (CallFunction|Boom))))

(event Custom|Boom
  ;[0 0 1] Explosion
  (Variables|Grenade|SetGrenadeLocation (Transformation|GetActorLocation self))
  (Variables|Boolean|SetHasDetonate true)
  (CallFunction|ExplosionSound)
  ;[0 1 0] Spawn FX
  (Default|Explosion (Variables|FX|GetFX_Manager) (Transformation|GetWorldLocation (Variables|Default|GetExplosionSphere)) 2.5 false true)
  ;[1 0 1] Explosion Sphere Timeline
  (bind _explosionsphereradiuspercentage (Timeline|ExplosionTimeline PlayFromStart)
    (:Update
      (Components|Sphere|SetSphereRadius (Variables|Default|GetExplosionSphere) (* _explosionsphereradiuspercentage (Variables|Blast|GetBlastRadius)) true)
      ;[0 0 1] Explose destructible mesh
      (Utilities|FlowControl|DoOnce false
        (:Completed
          (CallFunction|ExplosionDestructibleMesh))))
    (:Finished
      (Actor|DestroyActor))))

(event EventBeginPlay
  ;[1 0 0] Set time before explosion
  (Utilities|Time|SetTimerbyEvent (delegate Custom|Boom) (Variables|Grenade|GetTimeBeforeExplosion))
  ;[1 1 0] Add rotation to grande when thrown
  (Class|PrimitiveComponent|AddAngularImpulseinDegrees (Variables|Default|GetGrenadeMesh) "1000.000000, 0, 0" "None" true))

(event EventTick
  (params (DeltaSeconds :type Float%20%28single-precision%29)))

(fn ConstructionScript
  (Variables|/Script/Engine.ProjectileMovementComponent|SetBounciness (Variables|Grenade|GetProjectileMovement) (Variables|Grenade|GetBounciness))
  (Variables|/Script/Engine.ProjectileMovementComponent|SetFriction (Variables|Grenade|GetProjectileMovement) (Variables|Grenade|GetFriction))
  (Variables|/Script/Engine.ProjectileMovementComponent|SetInitialSpeed (Variables|Grenade|GetProjectileMovement) (Variables|Grenade|GetInitialSpeed))
  (Variables|/Script/Engine.ProjectileMovementComponent|SetMaxSpeed (Variables|Grenade|GetProjectileMovement) (Variables|Grenade|GetMaxSpeed)))

(fn Initialize
  (params (Fps%20Chara :type FPS%20Character%20Animated%20Object%20Reference))
  (Variables|Player|SetPlayer Fps%20Chara))

(fn ExplosionSound
  (Audio|SpawnSoundatLocation "/Game/SFX/MC/WEAPON/ATTACK/GRENADE/SFX_MC_WEA_ATK_Grenade_Explosion/SFX_MC_WEA_GrenadeExplosion_V01.SFX_MC_WEA_GrenadeExplosion_V01" (Transformation|GetWorldLocation (Variables|Default|GetGrenadeMesh)) "0, 0, 0" 3.0 1.0 0.0 0 0)
  (Components|DestroyComponent (Variables|Default|GetGrenadeMesh)))

(fn ExplosionRadiusOverlap
  (params (ActorOverlapped :type Actor%20Object%20Reference) (ExplosionLocation :type Vector))
  ;[1 0 0] Check actor is overlap
  (if (Utilities|Array|ContainsItem (Variables|Blast|GetActorOverlapped) (Utilities|GetClass ActorOverlapped))
    ;[0 1 1] It is the player ?
    (if (== ActorOverlapped (Variables|Player|GetPlayer))
      (if (Variables|Boolean|GetFriendlyFire)
        (Default|ShoottoPlayer (Variables|Player|GetPlayer) ExplosionLocation "0, 0, 0" (Variables|Grenade|GetDamage) false)
        ;[0 0 1] Explosion
        (Class|ShootInterface|Explose(Message) ActorOverlapped ExplosionLocation :!label _label))
      (else
        (goto _label)))))

(fn ExplosionDestructibleMesh
  (bind _returnvalue (AddComponent|AddRadialForceComponent true))
  (Transformation|AttachComponentToComponent _returnvalue (Variables|Default|GetGrenadeMesh) "None" "SnapToTarget" "KeepRelative" "KeepRelative" true)
  (Components|Activation|Activate _returnvalue true)
  (Variables|/Script/Engine.RadialForceComponent|SetRadius _returnvalue 5e+02)
  (Class|RadialForceComponent|FireImpulse _returnvalue))