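; Grenade pickup actor that the player collects by walking into it.
; On BeginPlay it finds and caches the FPS_Character_Animated in the level if no valid player reference is set.
; When CubeCollisionBox overlaps that player, it calls GrenadePickUp on the character, which handles the pickup, then destroys itself.
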(event OnComponentBeginOverlap(CubeCollisionBox)
  (params (OverlappedComponent :type Primitive%20Component%20Object%20Reference) (OtherActor :type Actor%20Object%20Reference) (OtherComp :type Primitive%20Component%20Object%20Reference) (OtherBodyIndex :type Integer) (bFromSweep :type Boolean) (SweepResult :type Hit%20Result%20Structure%20%28by%20ref%29))
  ;[0 0 1] Check if we have overlap the player
  (if (== OtherActor (Variables|Player|GetPlayer))
    (Default|GrenadePickUp (Variables|Player|GetPlayer))
    (Actor|DestroyActor)))

(event EventBeginPlay
  ;[0 0 1] Set player
  (Utilities|IsValid (Variables|Player|GetPlayer)
    (:Is%20Not%20Valid
      (bind _returnvalue (Actor|GetActorOfClass "/Game/MC/BP/FPS_Character_Animated.FPS_Character_Animated_C"))
      (Variables|Player|SetPlayer _returnvalue))))

(fn ConstructionScript)