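; Player controller for replay playback, which starts the replay paused with a UI when it is the local first controller.
; Gamepad buttons restart, pause or resume, change speed, jump in time and toggle the UI, calling replay functions defined outside this graph.
; Restarts and time jumps made while paused re-pause after a short delay, and Tick keeps the current demo time updated.
; Logic to match yaw to the character camera is disconnected.
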(event EventTick
  (params (DeltaSeconds :type Float%20%28single-precision%29))
  ;[1 0 0] Event tick - Update CurrentTime
  (CallFunction|UpdateCurrentTime))

(event EventBeginPlay
  ;[0 0 1] Replay - Begin play
  (bind _output_get (Variables|Default|SetIsControlled (== (Game|GetPlayerController 0) self)))
  (if _output_get
    (CallFunction|CreateUI)
    (Variables|Default|SetReplayPlayerState (Variables|Default|GetPlayerState))
    ;;[1 0 0] We start paused
    (Class|MyReplayPlayerController|RestartRecording)
    (Utilities|FlowControl|Delay 0.05)
    (CallFunction|PauseAfterAction)))

(event Input|GamepadEvents|GamepadFaceButtonLeft
  (params (Key :type Key%20Structure :default "None"))
  ;[1 0 0] Replay commands
  (:Pressed
    (if (Variables|Default|GetUIActive)
      ;;[0 0 1] Remove UI
      (Widget|RemovefromParent (Variables|Default|GetReplayUI))
      (Variables|Default|SetUIActive false)
      (else
        (CallFunction|CreateUI)
        (Variables|Default|SetUIActive true)))))

(event Input|GamepadEvents|GamepadDPadUp
  (params (Key :type Key%20Structure :default "None"))
  ;[1 0 0] Replay commands
  (:Pressed
    (Class|MyReplayPlayerController|IncreaseSpeedReplay)))

(event Input|GamepadEvents|GamepadDPadLeft
  (params (Key :type Key%20Structure :default "None"))
  ;[1 0 0] Replay commands
  (:Pressed
    (Class|MyReplayPlayerController|GoBackwardinTime)
    (if (Variables|Default|GetIsPaused)
      (Utilities|FlowControl|Delay 0.05)
      (CallFunction|PauseAfterAction))))

(event Input|GamepadEvents|GamepadDPadRight
  (params (Key :type Key%20Structure :default "None"))
  ;[1 0 0] Replay commands
  (:Pressed
    (Class|MyReplayPlayerController|GoForwardinTime)
    (if (Variables|Default|GetIsPaused)
      (Utilities|FlowControl|Delay 0.05)
      (CallFunction|PauseAfterAction))))

(event Input|GamepadEvents|GamepadFaceButtonRight
  (params (Key :type Key%20Structure :default "None"))
  ;[1 0 0] Replay commands
  (:Pressed
    (Class|MyReplayPlayerController|RestartRecording)
    (Utilities|FlowControl|Delay 0.2)
    (CallFunction|PauseAfterAction)))

(event Input|GamepadEvents|GamepadFaceButtonBottom
  (params (Key :type Key%20Structure :default "None"))
  ;[1 0 0] Replay commands
  (:Pressed
    (if (Variables|Default|GetIsPaused)
      (Class|MyReplayPlayerController|ResumeReplay)
      (Variables|Default|SetIsPaused false)
      (else
        (CallFunction|PauseAfterAction)))))

(event Input|GamepadEvents|GamepadDPadDown
  (params (Key :type Key%20Structure :default "None"))
  ;[1 0 0] Replay commands
  (:Pressed
    (Class|MyReplayPlayerController|DecreaseSpeedReplay)))

(event Input|GamepadEvents|GamepadFaceButtonTop
  (params (Key :type Key%20Structure :default "None"))
  ;[1 0 0] Replay commands
  (:Pressed
    (Class|MyReplayPlayerController|NormalSpeedReplay)))

(fn ConstructionScript)

(fn SetFPSCharacter
  (bind _returnvalue (Actor|GetActorOfClass "/Game/MC/BP/FPS_Character_Animated.FPS_Character_Animated_C"))
  (Variables|Default|SetFPS_Character _returnvalue))

(fn UpdateCurrentTime
  (bind _returnvalue (Class|MyReplayPlayerController|GetDemoCurrentTime))
  (Variables|Default|SetCurrentTime _returnvalue))

(fn Restart)

(fn PauseAfterAction
  (Class|MyReplayPlayerController|PauseReplay (Variables|Default|GetReplayPlayerState))
  (Variables|Default|SetIsPaused true))

(fn CreateUI
  (bind _returnvalue (UserInterface|CreateWidget "/Game/DataCollection/Replay/ReplayUI.ReplayUI_C"))
  (bind _output_get (Variables|Default|SetReplayUI _returnvalue))
  (UserInterface|Viewport|AddtoViewport _output_get 0))