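; BP_ReplaySpectatorPawn is a replay spectator pawn that follows the recorded first-person character's camera.
; It looks up the FPS_Character_Animated actor on BeginPlay and retries from Tick whenever that reference is invalid.
; Each tick it moves to the character's camera view location and sets its controller rotation to the camera's yaw only, zeroing pitch and roll.
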(event EventBeginPlay
  ;[1 0 0] Begin play  - Get FPS Character
  (CallFunction|SetFpsCharacter))

(event EventTick
  (params (DeltaSeconds :type Float%20%28single-precision%29))
  (CallFunction|SetPlayerReplayLocation))

(fn ConstructionScript)

(fn SetFpsCharacter
  (bind _returnvalue (Actor|GetActorOfClass "/Game/MC/BP/FPS_Character_Animated.FPS_Character_Animated_C"))
  (Utilities|IsValid _returnvalue
    (:Is%20Valid
      (Variables|Default|SetFPS_Character _returnvalue))))

(fn SetPlayerReplayLocation
  (bind _fps_character (Variables|Default|GetFPS_Character))
  (Utilities|IsValid _fps_character
    (:Is%20Valid
      _)
    (:Is%20Not%20Valid
      (CallFunction|SetFpsCharacter)))
  (bind _desiredview (Class|CameraComponent|GetCameraView (Variables|/Game/MC/BP/FPS_Character_Animated.FPS_Character_Animated_C|GetCamera _fps_character) 0.0))
  (Transformation|SetActorLocation (.location _desiredview) false false)
  (Pawn|SetControlRotation (Pawn|GetController) (Math|Rotator|MakeRotator 0.0 0.0 (.Yaw (Math|Rotator|BreakRotator (.rotation _desiredview))))))