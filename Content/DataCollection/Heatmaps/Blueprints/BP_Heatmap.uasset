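; Heatmap actor that records gameplay data for player, AI and destructible elements into render targets.
; Tick stamps the player's position, while custom events stamp shots, ledge grabs, hits, swaps, AI positions and deaths, and destructions.
; World locations are mapped into the actor's local space, scaled by resolution, and splatted through a dynamic material, with swaps drawn as color-lerped trails.
; Four render targets are cleared on BeginPlay and saved on EndPlay.
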(event Custom|Destructible%20Element%20-%20Draw%20to%20render%20Target
  (params (Location :type Vector))
  ;[0 1 0] Destructibles elements Data
  (Utilities|IsValid (Variables|Global|GetPlayer_Ref)
    (:Is%20Valid
      (CallFunction|DrawMaterialtoRenderTarget (Variables|SwapDestr|GetSize_DestrElem) (Variables|SwapDestr|GetStrength_DestrElem) (Variables|SwapDestr|GetRT_Runtime_SwapDestr) Location (Variables|SwapDestr|GetColor_DestElem)))))

(event Custom|Hit%20-%20Draw%20to%20render%20target
  ;[1 0 0] Player's Data
  ;;[1 0 0] Hit - Draw to render target
  (Utilities|IsValid (Variables|Global|GetPlayer_Ref)
    (:Is%20Valid
      (CallFunction|DrawMaterialtoRenderTarget (Variables|HitShootLedge|GetSize_Hit) (Variables|HitShootLedge|GetStrength_Hit) (Variables|HitShootLedge|GetRT_Hit_Shoot_Ledge) "0, 0, 0" (Variables|HitShootLedge|GetColor_Hit)))))

(event Custom|Shoot%20-%20Draw%20to%20render%20target
  ;[1 0 0] Player's Data
  ;;[1 0 0] Shoot - Draw to render target
  (Utilities|IsValid (Variables|Global|GetPlayer_Ref)
    (:Is%20Valid
      (CallFunction|DrawMaterialtoRenderTarget (Variables|HitShootLedge|GetSize_Shoot) (Variables|HitShootLedge|GetStrength_Shoot) (Variables|HitShootLedge|GetRT_Hit_Shoot_Ledge) "0, 0, 0" (Variables|HitShootLedge|GetColor_Shoot)))))

(event Custom|Ledge%20grap%20_Draw%20to%20render%20target
  ;[1 0 0] Player's Data
  ;;[1 0 0] Ledge grap - Draw to render target
  (Utilities|IsValid (Variables|Global|GetPlayer_Ref)
    (:Is%20Valid
      (CallFunction|DrawMaterialtoRenderTarget (Variables|HitShootLedge|GetSize_LedgeGrap) (Variables|HitShootLedge|GetStrength_LedgeGrap) (Variables|HitShootLedge|GetRT_Hit_Shoot_Ledge) "0, 0, 0" (Variables|HitShootLedge|GetColor_LedgeGrap)))))

(event Custom|Swap%20-%20Draw%20to%20render%20target
  (params (EndPosition :type Vector))
  ;[1 0 0] Player's Data
  ;;[1 0 0] Swap - Draw to render Target
  (Utilities|IsValid (Variables|Global|GetPlayer_Ref)
    (:Is%20Valid
      (Swap|SwapDrawing (Transformation|GetActorLocation (Variables|Global|GetPlayer_Ref)) EndPosition))))

(event Custom|AI%20Death%20-%20Draw%20to%20render%20target
  (params (Location :type Vector))
  ;[0 0 1] AI'S data
  ;;[0 0 1] AI Death - Draw to render target
  (Utilities|IsValid (Variables|Global|GetPlayer_Ref)
    (:Is%20Valid
      (CallFunction|DrawMaterialtoRenderTarget (Variables|AIDeathAIPosition|GetSize_AIDeath) (Variables|AIDeathAIPosition|GetStrength_AIDeath) (Variables|AIDeathAIPosition|GetRt_AIDeathAIPosition) Location (Variables|AIDeathAIPosition|GetColor_AIDeath)))))

(event Custom|AI%20Position%20-%20Draw%20to%20render%20target
  (params (Location :type Vector))
  ;[0 0 1] AI'S data
  ;;[0 0 1] AI Position - Draw to render target
  (Utilities|IsValid (Variables|Global|GetPlayer_Ref)
    (:Is%20Valid
      (CallFunction|DrawMaterialtoRenderTarget (Variables|AIDeathAIPosition|GetSize_AIPosition) (Variables|AIDeathAIPosition|GetStrength_AIPosition) (Variables|AIDeathAIPosition|GetRt_AIDeathAIPosition) Location (Variables|AIDeathAIPosition|GetColor_AIPosition)))))

(event EventBeginPlay
  ;[1 0 0] Begin Play - Initialize
  (Begin|InitializeHeatmap))

(event EventEndPlay
  (params (EndPlayReason :type EEndPlayReason%20Enum :default "Destroyed"))
  ;[1 0 0] End Play - Bake the map
  (Utilities|IsValid (Variables|Global|GetPlayer_Ref)
    (:Is%20Valid
      (End|ExportRenderTarget))))

(event EventTick
  (params (DeltaSeconds :type Float%20%28single-precision%29))
  ;[1 0 0] Player's Data
  ;;[1 0 0] Position - Draw to render Target
  (Utilities|IsValid (Variables|Global|GetPlayer_Ref)
    (:Is%20Valid
      (CallFunction|DrawMaterialtoRenderTarget (Variables|Position|GetSize_Position) (Variables|Position|GetStrength_Position) (Variables|Position|GetRT_Position) "0, 0, 0" (Variables|Position|GetColor_Position)))))

(fn ConstructionScript
  (bind _returnvalue (Rendering|Material|CreateDynamicMaterialInstance "/Game/DataCollection/Heatmaps/Materials/M_HeatSplat.M_HeatSplat" "None" "None" :!class /Script/Engine.KismetMaterialLibrary))
  (Variables|Global|SetMID_HeatSplat _returnvalue))

(fn InitializeHeatmap
  ;[1 0 0] Begin Play - Get player ref and clear render target 2D
  (Variables|Global|SetPlayer_Ref (Game|GetPlayerCharacter 0))
  (Variables|Default|SetDefaultResolution (Variables|Global|GetResolution))
  (Rendering|ClearRenderTarget2D (Variables|Position|GetRT_Position))
  (Rendering|ClearRenderTarget2D (Variables|HitShootLedge|GetRT_Hit_Shoot_Ledge))
  (Rendering|ClearRenderTarget2D (Variables|SwapDestr|GetRT_Runtime_SwapDestr))
  (Rendering|ClearRenderTarget2D (Variables|AIDeathAIPosition|GetRt_AIDeathAIPosition)))

(fn CanbeDrawn
  (bind _self self)
  (bind _player_ref (Variables|Global|GetPlayer_Ref))
  (bind _defaultsceneroot (Variables|Default|GetDefaultSceneRoot _self))
  (bind _returnvalue (Transformation|GetWorldLocation _defaultsceneroot))
  (Utilities|IsValid _player_ref
    (:Is%20Valid
      (bind _returnvalue_2 (Class|HeatmapCheckActorPosition|CheckPosition (Variables|Default|GetHeatmapCheckActorPosition) (Math|Conversions|ToVector2D(Vector) (Transformation|GetActorLocation _player_ref)) (Math|Conversions|ToVector2D(Vector) _returnvalue) (|CalculMaxPosition_2 _returnvalue)))
      (if _returnvalue_2
        (CallFunction|DrawMaterialtoRenderTarget (Variables|Position|GetSize_Position) (Variables|Position|GetStrength_Position) (Variables|Position|GetRT_Position) "0, 0, 0")))))

(fn DrawMaterialtoRenderTarget
  (params (Size :type Float%20%28single-precision%29) (Strength :type Float%20%28single-precision%29) (RenderTargetRuntime :type Texture%20Render%20Target%202D%20Object%20Reference) (Location :type Vector) (FinalColor :type Linear%20Color%20Structure))
  ;[1 0 0] If no value is given, we take the player's position
  (if (Math|Vector|Equal(Vector) Location "0, 0, 0" 0.0001)
    ;[0 0 1] No Location given
    (Class|Heatmap|DrawtoRenderTargetFunction (Math|Conversions|ToLinearColor(Vector) (|PositionfromworldtoRenderTarget (Transformation|GetActorLocation (Variables|Global|GetPlayer_Ref)))) FinalColor Size Strength RenderTargetRuntime (Variables|Global|GetMID_HeatSplat))
    (else
      ;[0 1 1] Location given
      (Class|Heatmap|DrawtoRenderTargetFunction (Math|Conversions|ToLinearColor(Vector) (|PositionfromworldtoRenderTarget_2 Location)) FinalColor Size Strength RenderTargetRuntime (Variables|Global|GetMID_HeatSplat)))))

(fn IncreaseAlphaSwap
  ;[1 0 1] Increase value for while loop
  (Variables|SwapDestr|SetAlpha_Swap (+ (Variables|SwapDestr|GetAlpha_Swap) 0.08)))

(fn SwapDrawing
  (params (StartPosition :type Vector) (EndPosition :type Vector))
  ;[0 0 1] Prepare While Loop
  (Variables|SwapDestr|SetAlpha_Swap 0.0)
  (Variables|SwapDestr|SetStrength_Swap 2e+02)
  (while (< (Variables|SwapDestr|GetAlpha_Swap) 1.0)
    ;[1 0 0] Update strength for it to get more red
    (Variables|SwapDestr|SetStrength_Swap (+ (Variables|SwapDestr|GetStrength_Swap) 5e+01))
    (CallFunction|DrawMaterialtoRenderTarget (Variables|SwapDestr|GetSize_Swap) (Variables|SwapDestr|GetStrength_Swap) (Variables|SwapDestr|GetRT_Runtime_SwapDestr) (Math|Vector|Lerp(Vector) StartPosition EndPosition (Variables|SwapDestr|GetAlpha_Swap)) (Math|Color|Lerp(LinearColor) (Variables|SwapDestr|GetBegin_Color_Swap) (Variables|SwapDestr|GetFinal_Color_Swap) (Variables|SwapDestr|GetAlpha_Swap)))
    (Swap|IncreaseAlphaSwap)))

(fn ExportRenderTarget
  (Class|Heatmap|PrepareSaveRenderTarget)
  (Class|Heatmap|SaveRenderTarget (Variables|Position|GetRT_Position))
  (Class|Heatmap|SaveRenderTarget (Variables|HitShootLedge|GetRT_Hit_Shoot_Ledge))
  (Class|Heatmap|SaveRenderTarget (Variables|SwapDestr|GetRT_Runtime_SwapDestr))
  (Class|Heatmap|SaveRenderTarget (Variables|AIDeathAIPosition|GetRt_AIDeathAIPosition)))